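; Weeping-angel style intruder AI that advances on the first-person player only while unseen and jumpscares on contact.
; Each tick, a behind-camera check, a visibility trace and the player's blink state drive the CanMove blackboard key and movement mode.
; Capsule hits while the player blinks or faces away fire a one-time scare: camera turn, spotlight, shake, sound and fade to black.
; A looping timer plays attached breathing sounds.
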(event OnComponentHit(CapsuleComponent)
  (params (HitComponent :type Primitive%20Component%20Object%20Reference) (OtherActor :type Actor%20Object%20Reference) (OtherComp :type Primitive%20Component%20Object%20Reference) (NormalImpulse :type Vector :default "0, 0, 0") (Hit :type Hit%20Result%20Structure%20%28by%20ref%29))
  (bind _returnvalue (Game|GetPlayerController 0))
  (bind _firstperson (Variables|Default|GetFirstperson))
  ;[1 1 1] Jumpscare
  (Utilities|Casting|CastToBP_FirstPersonCharacter OtherActor)
  (if (Variables|/Game/FirstPerson/Blueprints/BP_FirstPersonCharacter.BP_FirstPersonCharacter_C|GetIsBlinking? (Variables|Default|GetFirstperson))
    (Utilities|FlowControl|Delay 0.35))
  (if (or (Variables|/Game/FirstPerson/Blueprints/BP_FirstPersonCharacter.BP_FirstPersonCharacter_C|GetIsBlinking? (Variables|Default|GetFirstperson)) (Variables|Default|GetBehind%20Anchor))
    (Utilities|FlowControl|DoOnce false
      (:Completed
        (Audio|PlaySound2D "/Game/SFX/jumpscareSFX.jumpscareSFX" 1.0 1.0 0.0 0 0)
        (Pawn|SetControlRotation _returnvalue (Math|Interpolation|RInterpTo (Pawn|GetControlRotation _returnvalue :!class /Script/Engine.Controller) (Math|Rotator|FindLookatRotation (Transformation|GetActorLocation (Variables|Default|GetFirstperson)) (Transformation|GetWorldLocation (Variables|Default|GetSphere))) 1.0 4.0))
        (if (Variables|/Game/FirstPerson/Blueprints/BP_FirstPersonCharacter.BP_FirstPersonCharacter_C|GetIsBlinking? _firstperson)
          (Default|OpeningEyes (Variables|/Game/FirstPerson/Blueprints/BP_FirstPersonCharacter.BP_FirstPersonCharacter_C|GetBlink%20Widget _firstperson)))
        (Transformation|SetActorRotation (Math|Rotator|FindLookatRotation (Transformation|GetActorLocation self) (Transformation|GetActorLocation (Variables|Default|GetFirstperson))))
        (Pawn|Components|CharacterMovement|DisableMovement (Variables|/Script/Engine.Character|GetCharacterMovement (Variables|Default|GetFirstperson)))
        (Rendering|SetVisibility (Variables|Default|GetSpotLight) true false)
        (Variables|Default|GetFadetoblack
          (:then
            _)
          (:else
            (bind _returnvalue_2 (UserInterface|CreateWidget "/Game/BP_BLink/UI/BPW_FadetoBlack.BPW_FadetoBlack_C"))
            (bind _output_get (Variables|Default|SetFadetoblack _returnvalue_2))))
        (UserInterface|Viewport|AddtoViewport _output_get 0)
        (Default|FadesTOblack (Variables|Default|GetFadetoblack))
        (CameraShakes|StartCameraShake (Game|GetPlayerCameraManager 0) "/Game/BP_BLink/BP_jumpscareShake.BP_jumpscareShake_C" 1.0 "CameraLocal" "0, 0, 0")
        (Audio|Components|Audio|Stop (Variables|/Game/FirstPerson/Blueprints/BP_FirstPersonCharacter.BP_FirstPersonCharacter_C|GetFootSteps_TL (Variables|Default|GetFirstperson)))))))

(event Custom|CheckBreathing
  (Utilities|IsValid (Variables|Default|GetFirstperson)
    (:Is%20Valid
      (if (Variables|Default|GetDelay)
        (Audio|SpawnSoundAttached "/Game/SFX/BreathingSFX.BreathingSFX" (Variables|Character|GetMesh) "None" "0, 0, 0" "0, 0, 0" "KeepRelativeOffset" false 1.0 1.0 0.0 0 0)
        (Variables|Default|SetDelay false)
        (Utilities|FlowControl|Delay 1.0)
        (Variables|Default|SetDelay true)))))

(event Custom|WeepingAngel
  (bind _first_person_camera (Variables|Default|GetFirst%20Person%20Camera))
  (bind _charactermovement (Variables|Character|GetCharacterMovement))
  ;[1 1 1] Intruder set Movement
  (Utilities|IsValid (Variables|Default|GetFirstperson)
    (:Is%20Valid
      (bind _behindanchor (CallFunction|LocationBehindActorCheck (Transformation|GetWorldLocation _first_person_camera) (Transformation|GetWorldRotation _first_person_camera) (Transformation|GetActorLocation)))
      (Variables|Default|SetBehind%20Anchor _behindanchor)
      (bind _outhit (Collision|LineTraceByChannel (Transformation|GetWorldLocation (Variables|Default|GetFirst%20Person%20Camera)) (Transformation|GetWorldLocation (Variables|Default|GetSphere1)) "TraceTypeQuery1" false 0 "None" false))
      (if (Math|Boolean|ORBoolean (Variables|Default|GetBehind%20Anchor) (not (== (.HitActor (Collision|BreakHitResult _outhit)) self)) (Variables|/Game/FirstPerson/Blueprints/BP_FirstPersonCharacter.BP_FirstPersonCharacter_C|GetIsBlinking? (Variables|Default|GetFirstperson)))
        (AI|Components|Blackboard|SetValueasBool (AI|GetBlackboard 0) (Utilities|Name|MakeLiteralName "CanMove") true)
        (Utilities|FlowControl|Delay 0.2)
        (Pawn|Components|CharacterMovement|SetMovementMode _charactermovement "MOVE_NavWalking" 0)
        (Development|PrintString "MOve" true true "(R=0.000000,G=0.660000,B=1.000000,A=1.000000)" 2.0 "fthjfth")
        (else
          (AI|Components|Blackboard|SetValueasBool (AI|GetBlackboard 0) (Utilities|Name|MakeLiteralName "CanMove") false)
          (Pawn|Components|CharacterMovement|SetMovementMode _charactermovement "MOVE_None" 0)
          (Development|PrintString "Stop" true true "(R=0.000000,G=0.660000,B=1.000000,A=1.000000)" 2.0 "srujrj"))))))

(event EventTick
  (params (DeltaSeconds :type Float%20%28single-precision%29))
  (CallFunction|WeepingAngel))

(event EventBeginPlay
  (Utilities|Time|SetTimerbyFunctionName 0 "CheckBreathing" 4.0 true)
  (bind _returnvalue (Actor|GetActorOfClass "/Game/FirstPerson/Blueprints/BP_FirstPersonCharacter.BP_FirstPersonCharacter_C"))
  (Variables|Default|SetFirst%20Person%20Camera (Variables|/Game/FirstPerson/Blueprints/BP_FirstPersonCharacter.BP_FirstPersonCharacter_C|GetFirstPersonCamera _returnvalue))
  (Variables|Default|SetFirstperson _returnvalue))

(fn ConstructionScript)