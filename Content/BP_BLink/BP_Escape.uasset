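; BP_Escape is a trigger actor that ends the game with an escape win when the first-person player reaches it.
; When BP_FirstPersonCharacter overlaps its Box, it creates the BPW_Win widget once, adds it to the viewport and plays its EscapeFade.
; It then disables the character's movement and stops its footstep timeline.
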(event OnComponentBeginOverlap(Box)
  (params (OverlappedComponent :type Primitive%20Component%20Object%20Reference) (OtherActor :type Actor%20Object%20Reference) (OtherComp :type Primitive%20Component%20Object%20Reference) (OtherBodyIndex :type Integer) (bFromSweep :type Boolean) (SweepResult :type Hit%20Result%20Structure%20%28by%20ref%29))
  (bind _asbp_first_person_character (Utilities|Casting|CastToBP_FirstPersonCharacter OtherActor))
  (Variables|Default|SetAs%20BP%20First%20Person%20Character _asbp_first_person_character)
  (Variables|Default|GetWin
    (:then
      _)
    (:else
      (bind _returnvalue (UserInterface|CreateWidget "/Game/BP_BLink/UI/BPW_Win.BPW_Win_C"))
      (bind _output_get (Variables|Default|SetWin _returnvalue))))
  (UserInterface|Viewport|AddtoViewport _output_get 0)
  (Default|EscapeFade (Variables|Default|GetWin))
  (Pawn|Components|CharacterMovement|DisableMovement (Variables|/Script/Engine.Character|GetCharacterMovement (Variables|Default|GetAs%20BP%20First%20Person%20Character)))
  (Audio|Components|Audio|Stop (Variables|/Game/FirstPerson/Blueprints/BP_FirstPersonCharacter.BP_FirstPersonCharacter_C|GetFootSteps_TL (Variables|Default|GetAs%20BP%20First%20Person%20Character))))

(event EventBeginPlay)

(event Collision|EventActorBeginOverlap
  (params (OtherActor :type Actor%20Object%20Reference)))

(event EventTick
  (params (DeltaSeconds :type Float%20%28single-precision%29)))

(fn ConstructionScript)