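; BP_Door is an interactable door that swings open and closed on alternate interactions.
; OnInteract uses a FlipFlop to play one timeline forward from the start or a second timeline in reverse from the end.
; Each timeline's DoorOPen track drives the Door component's relative yaw.
; The IsOpenIng flag ignores further interactions until the current swing finishes.
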(event EventBeginPlay)

(event Collision|EventActorBeginOverlap
  (params (OtherActor :type Actor%20Object%20Reference)))

(event EventTick
  (params (DeltaSeconds :type Float%20%28single-precision%29)))

(event EventOnInteract
  (bind _door (Variables|Default|GetDoor))
  (if (not (Variables|Default|GetIsOpenIng?))
    (Variables|Default|SetIsOpenIng? true)
    (Utilities|FlowControl|FlipFlop
      (:A
        (bind _dooropen (Timeline|Timeline PlayFromStart)
          (:Update
            (Transformation|SetRelativeRotation _door (Math|Rotator|MakeRotator 0.0 0.0 _dooropen) false false))
          (:Finished
            (Variables|Default|SetIsOpenIng? false))))
      (:B
        (bind _dooropen_2 (Timeline|Timeline_0 ReverseFromEnd)
          (:Update
            (Transformation|SetRelativeRotation _door (Math|Rotator|MakeRotator 0.0 0.0 _dooropen_2) false false))
          (:Finished
            (Variables|Default|SetIsOpenIng? false)))))))

(fn ConstructionScript)